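; Game state Blueprint that saves and restores the transforms of world actors through a single fixed save slot.
; SaveGame records the reference, class and transform of every actor implementing the SaveGameObject interface into a new BP_SaveGameData.
; LoadGame reads that data back, moving actors whose references still resolve and spawning the saved class at the saved transform for the rest.
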(fn `LoadGame`
  (locals (SaveData :type "/Game/SaveGameExample/BP_SaveGameData Object Reference"))
  (`|ExecutionSequence`
    (:`then_0`
      (bind _returnvalue (`GameplayStatics.LoadGameFromSlot` "SaveGame"))
      (bind _asbp_save_game_data (cast `/Game/SaveGameExample/BP_SaveGameData` _returnvalue))
      (set `local.SaveData` _asbp_save_game_data))
    (:`then_1`
      (bind _savedata (`local.SaveData`)
        (:`then`
          (for _array_element (`/Game/SaveGameExample/BP_SaveGameData.ActorData` _savedata)
            (bind (_actor _class _transform) (break `/Game/SaveGameExample/Structs/SaveGameActorData` _array_element))
            (bind _output (`|ConvertAsset` _actor))
            (`/Engine/EditorBlueprintResources/StandardMacros.IsValid` _output
              (:`Is Valid`
                (`self.K2_SetActorTransform` _output _transform false false))
              (:`Is Not Valid`
                (`|SpawnActorFromClass` (`|ConvertAsset` _class) _transform "AlwaysSpawn" "MultiplyWithRoot" null null)))))
        (:`else`)))))

(fn `SaveGame`
  (locals (SaveData :type "/Game/SaveGameExample/BP_SaveGameData Object Reference"))
  (`|ExecutionSequence`
    (:`then_0`
      (bind _returnvalue (`GameplayStatics.CreateSaveGameObject` "/Game/SaveGameExample/BP_SaveGameData.BP_SaveGameData_C"))
      (set `local.SaveData` _returnvalue))
    (:`then_1`
      (bind _outactors (`GameplayStatics.GetAllActorsWithInterface` "/Script/SaveGamePlugin.SaveGameObject"))
      (for _array_element _outactors
        (`KismetArrayLibrary.Array_Add` (`/Game/SaveGameExample/BP_SaveGameData.ActorData` (`local.SaveData`)) (make `/Game/SaveGameExample/Structs/SaveGameActorData` (`|ConvertAsset` _array_element) (`|ConvertAsset` (`GameplayStatics.GetObjectClass` _array_element)) (`self.GetTransform` _array_element)))))
    (:`then_2`
      (`GameplayStatics.SaveGameToSlot` (`local.SaveData`) "SaveGame"))))

(fn `UserConstructionScript`)